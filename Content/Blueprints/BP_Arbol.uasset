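; BP_Arbol is a tree actor that continuously produces BP_Madera wood pieces.
; On BeginPlay it spawns an initial burst of wood, then repeats GenerarMadera indefinitely on a one-second delay loop.
; Each piece spawns at the Generador component's transform and gets a strong impulse in a random direction on its Cube, scattering it outward.
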(event Custom|GenerarMadera
  (bind _returnvalue (Game|SpawnActorfromClass "/Game/Blueprints/BP_Madera.BP_Madera_C" (Transformation|GetWorldTransform (Variables|Default|GetGenerador)) "Undefined" "MultiplyWithRoot" 0 0))
  (Physics|AddImpulse (Variables|/Game/Blueprints/BP_Madera.BP_Madera_C|GetCube _returnvalue) (* (Math|Random|RandomUnitVector) 2e+04) "None" false))

(event EventBeginPlay
  (for _index (range 0 5)
    (CallFunction|GenerarMadera))
  (CallFunction|GenerarMadera :!label _label)
  (Utilities|FlowControl|Delay 1.0)
  (goto _label))

(fn ConstructionScript)