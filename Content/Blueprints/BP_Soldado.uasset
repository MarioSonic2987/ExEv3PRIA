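; BP_Soldado is a soldier Blueprint that colors its mesh according to its faction.
; Its construction script calls the parent version, then creates a dynamic instance of MI_Manny_02 on the mesh's first material slot.
; It sets that material's Tint parameter to the color GetColorFaccion returns for Faccion.
; The event graph holds only disabled default events, so it adds no gameplay logic there.
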(event EventBeginPlay
  (|CallParentFunction) ; This node is disabled and will not be called.\nDrag off pins to build functionality.
)

(event Collision|EventActorBeginOverlap
  (params (OtherActor :type Actor%20Object%20Reference))
  (|CallParentFunction OtherActor) ; This node is disabled and will not be called.\nDrag off pins to build functionality.
)

(event EventTick
  (params (DeltaSeconds :type Float%20%28single-precision%29))
  (|CallParentFunction DeltaSeconds) ; This node is disabled and will not be called.\nDrag off pins to build functionality.
)

(fn ConstructionScript
  (|CallParentFunction)
  (bind _returnvalue (Rendering|Material|CreateDynamicMaterialInstance (Variables|Character|GetMesh) 0 "/Game/Characters/Mannequins/Materials/Instances/Manny/MI_Manny_02.MI_Manny_02" "None" :!class /Script/Engine.PrimitiveComponent))
  (Rendering|Material|SetVectorParameterValue _returnvalue "Tint" (CallFunction|GetColorFaccion (Variables|Default|GetFaccion)) :!class /Script/Engine.MaterialInstanceDynamic))