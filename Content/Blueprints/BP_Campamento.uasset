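; BP_Campamento is a faction camp that keeps spawning actors for its faction during play.
; From BeginPlay it loops endlessly, waiting a random few seconds, then spawning the configured class at its own transform and passing on its faction.
; The construction script tints the roof tiles with the faction color through a dynamic material instance on the static mesh.
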(event EventBeginPlay
  (|CallParentFunction)
  (Utilities|FlowControl|Delay (Math|Random|RandomFloatinRange 5.0 1e+01) :!label _label)
  (Game|SpawnActorfromClass (Variables|Default|GetClaseAGenerar) (Transformation|GetActorTransform) "Undefined" "MultiplyWithRoot" 0 (Variables|Default|GetFaccion) 0)
  (goto _label))

(fn ConstructionScript
  (|CallParentFunction)
  (bind _returnvalue (Rendering|Material|CreateDynamicMaterialInstance (Variables|Default|GetStaticMesh) 3 "/Game/Fantastic_Village_Pack/materials/MI_rooftiles_01.MI_rooftiles_01" "None" :!class /Script/Engine.PrimitiveComponent))
  (Rendering|Material|SetVectorParameterValue _returnvalue "Base Color Tint" (CallFunction|GetColorFaccion (Variables|Default|GetFaccion)) :!class /Script/Engine.MaterialInstanceDynamic))